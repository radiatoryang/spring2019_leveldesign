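; MyPlayerCharacter is the player-controlled character, with a countdown that serves as the lose condition.
; Input axis and action events drive movement along the actor's forward and right vectors, controller look, and jumping.
; BeginPlay creates MyHUDWidget and adds it to the viewport.
; Tick reduces TimeLeft by delta time and, once it reaches zero, prints a losing message every frame without ending play.
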(event `InputAxis|MoveForward`
  (params (AxisValue :type "Float (single-precision)"))
  (`self.AddMovementInput` (`self.GetActorForwardVector`) AxisValue))

(event `InputAxis|LookUp`
  (params (AxisValue :type "Float (single-precision)"))
  (`self.AddControllerPitchInput` AxisValue))

(event `self.ReceiveBeginPlay`
  (bind _returnvalue (`|CreateWidget` "/Game/Blueprints/MyHUDWidget.MyHUDWidget_C")) ; initialize the HUD Widget object
  (`UserWidget.AddToViewport` _returnvalue 0) ; add HUD to viewport
)

(event `InputAction|JumpAction`
  (params (Key :type "Key Structure"))
  (:`Pressed`
    (`self.Jump`))
  (:`Released`
    (`self.StopJumping`)))

(event `InputAxis|LookRight`
  (params (AxisValue :type "Float (single-precision)"))
  (`self.AddControllerYawInput` AxisValue))

(event `InputAxis|MoveRight`
  (params (AxisValue :type "Float (single-precision)"))
  (`self.AddMovementInput` (`self.GetActorRightVector`) AxisValue))

(event `self.ReceiveTick`
  (params (DeltaSeconds :type "Float (single-precision)"))
  (bind _output_get (set `self.TimeLeft` (- (`self.TimeLeft`) DeltaSeconds)))
  (if (<= _output_get 0.0)
    (`KismetSystemLibrary.PrintString` "You are a loser")))

(fn `UserConstructionScript`)